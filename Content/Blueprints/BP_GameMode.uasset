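; Game mode that resolves damage between players.
; OnPlayerDamage subtracts the attacker's PlayerState Damage from the victim's PlayerState HP, clamps it at zero and calls RefreshPlayerHp on the victim's state.
; It returns true when the victim's HP is depleted.
; BeginPlay, the construction script and GetHP are empty.
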(event EventBeginPlay)

(fn ConstructionScript)

(fn OnPlayerDamage
  (params (Attacker :type BP%20Player%20Object%20Reference) (Victim :type BP%20Human%20Object%20Reference))
  (bind _asbp_player_state (Utilities|Casting|CastToBP_PlayerState (Variables|/Script/Engine.Pawn|GetPlayerState Victim)))
  (bind _asbp_player_state_2 (Utilities|Casting|CastToBP_PlayerState (Variables|/Script/Engine.Pawn|GetPlayerState Attacker)))
  (bind _output_get (Variables|/Game/Blueprints/Character/Player/BP_PlayerState.BP_PlayerState_C|SetHP _asbp_player_state (Math|Integer|Max(Integer) (- (Variables|/Game/Blueprints/Character/Player/BP_PlayerState.BP_PlayerState_C|GetHP _asbp_player_state) (Variables|/Game/Blueprints/Character/Player/BP_PlayerState.BP_PlayerState_C|GetDamage _asbp_player_state_2)))))
  (Default|RefreshPlayerHp _asbp_player_state)
  (if (<= _output_get 0)
    (return true)))

(fn GetHP)