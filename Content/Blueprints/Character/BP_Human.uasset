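; BP_Human is a character Blueprint, castable to BP_Player, that handles melee hits and death.
; On authority, the attack-hit event sphere-traces toward the front for pawns, adds hits to HitHuman and damages each human there.
; When damaged while idle/moving or attacking, non-players die outright, while BP_GameMode's OnPlayerDamage also rules on player-caused hits.
; Death sets the Dead state, disables movement and capsule collision, and ragdolls the mesh.
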(event Custom|S2M_Death
  (bind _mesh (Variables|Character|GetMesh))
  (Utilities|FlowControl|Sequence
    (:then_0
      (Variables|Default|SetState "NewEnumerator2"))
    (:then_1
      (Pawn|Components|CharacterMovement|DisableMovement (Variables|Character|GetCharacterMovement)))
    (:then_2
      (Collision|SetCollisionEnabled (Variables|Collision|GetCapsuleComponent) "NoCollision"))
    (:then_3
      (Collision|SetCollisionEnabled _mesh "PhysicsOnly")
      (Physics|SetSimulatePhysics _mesh true))))

(event Game|Damage|EventAnyDamage
  (params (Damage :type Float%20%28single-precision%29) (DamageType :type Damage%20Type%20Object%20Reference) (InstigatedBy :type Controller%20Object%20Reference) (DamageCauser :type Actor%20Object%20Reference))
  (switch Utilities|FlowControl|Switch|SwitchonE_State (Variables|Default|GetState)
    (:NewEnumerator0
      _)
    (:NewEnumerator1
      _))
  (Utilities|FlowControl|Sequence
    (:then_0
      (Utilities|Casting|CastToBP_Player self
        (:CastFailed
          (CallFunction|S2MDeath))))
    (:then_1
      (bind _asbp_game_mode (Utilities|Casting|CastToBP_GameMode (Game|GetGameMode)))
      (bind _asbp_player (Utilities|Casting|CastToBP_Player DamageCauser))
      (bind _isdeath (Default|OnPlayerDamage _asbp_game_mode _asbp_player self))
      (if _isdeath
        (CallFunction|S2MDeath)))))

(event Custom|CallAttackHit
  (bind _returnvalue (Transformation|GetActorLocation))
  (Networking|SwitchHasAuthority
    (:Authority
      (bind _outhits (Collision|MultiSphereTraceForObjects (+ (* (Transformation|GetActorRightVector) -5e+01) _returnvalue) (+ _returnvalue (* (Transformation|GetActorForwardVector) (Variables|Default|GetAttackRange))) 15.0 (Utilities|Array|MakeArray "ObjectTypeQuery3") false 0 "None"))
      (for _array_element _outhits
        (Utilities|Array|AddUnique (Variables|Default|GetHitHuman) (.HitActor (Collision|BreakHitResult _array_element))))
      (for _array_element_2 (Variables|Default|GetHitHuman)
        (bind _asbp_human (Utilities|Casting|CastToBP_Human _array_element_2))
        (Game|Damage|ApplyDamage _asbp_human 2e+01 0 self)))))

(event Custom|CallAttackEnd
  (switch Utilities|FlowControl|Switch|SwitchonE_State (Variables|Default|GetState)
    (:NewEnumerator1
      (Variables|Default|SetState "NewEnumerator0"))))

(fn ConstructionScript)