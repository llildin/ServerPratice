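; Player controller that turns Enhanced Input into actions on the possessed BP_Player and creates the main HUD.
; BeginPlay caches the pawn, adds the default mapping context, then requests WBP_MainUI through a C2S-to-S2M event chain, seeding its HP from PlayerState.
; Look rotates the controller, movement follows control yaw, and jump, crouch and attack forward to the pawn, with attack firing on both Started and Triggered.
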(event Custom|C2S_CreateUI
  (CallFunction|S2MCreateUI))

(event Custom|S2M_CreateUI
  (bind _returnvalue (UserInterface|CreateWidget "/Game/UI/WBP_MainUI.WBP_MainUI_C"))
  (bind _output_get (Variables|Default|SetMainUI _returnvalue))
  (UserInterface|Viewport|AddtoViewport _output_get 0)
  (Default|SetHP _output_get (Variables|/Game/Blueprints/Character/Player/BP_PlayerState.BP_PlayerState_C|GetHP (Default|GetPlayerState (Variables|Default|GetPlayerRef)))))

(event Input|EnhancedActionEvents|EnhancedInputActionIA_Move
  (params (ActionValue :type Vector%202D%20Structure) (ElapsedSeconds :type Float%20%28double-precision%29) (TriggeredSeconds :type Float%20%28double-precision%29) (InputAction :type Input%20Action%20Object%20Reference :default "/Game/Assets/Input/Action/IA_Move.IA_Move"))
  (bind _returnvalue (Pawn|GetControlRotation :!class /Script/Engine.Controller))
  (bind (_x _y) (Math|Vector2D|BreakVector2D ActionValue))
  (bind _returnvalue_2 (Pawn|GetControlRotation :!class /Script/Engine.Controller))
  (Pawn|Input|AddMovementInput (Variables|Default|GetPlayerRef) (Math|Vector|GetForwardVector (Math|Rotator|MakeRotator (.roll _returnvalue) 0.0 (.yaw _returnvalue))) _y false)
  (Pawn|Input|AddMovementInput (Variables|Default|GetPlayerRef) (Math|Vector|GetRightVector (Math|Rotator|MakeRotator (.roll _returnvalue_2) 0.0 (.yaw _returnvalue_2))) _x false))

(event Input|EnhancedActionEvents|EnhancedInputActionIA_Look
  (params (ActionValue :type Vector%202D%20Structure) (ElapsedSeconds :type Float%20%28double-precision%29) (TriggeredSeconds :type Float%20%28double-precision%29) (InputAction :type Input%20Action%20Object%20Reference :default "/Game/Assets/Input/Action/IA_Look.IA_Look"))
  (bind (_x _y) (Math|Vector2D|BreakVector2D ActionValue))
  (Class|PlayerController|AddYawInput _x)
  (Class|PlayerController|AddPitchInput _y))

(event Input|EnhancedActionEvents|EnhancedInputActionIA_Jump
  (params (ActionValue :type Boolean) (ElapsedSeconds :type Float%20%28double-precision%29) (TriggeredSeconds :type Float%20%28double-precision%29) (InputAction :type Input%20Action%20Object%20Reference :default "/Game/Assets/Input/Action/IA_Jump.IA_Jump"))
  (bind _playerref (Variables|Default|GetPlayerRef))
  (:Started
    (Character|Jump _playerref))
  (:Completed
    (Character|StopJumping _playerref)))

(event Input|EnhancedActionEvents|EnhancedInputActionIA_Crouch
  (params (ActionValue :type Boolean) (ElapsedSeconds :type Float%20%28double-precision%29) (TriggeredSeconds :type Float%20%28double-precision%29) (InputAction :type Input%20Action%20Object%20Reference :default "/Game/Assets/Input/Action/IA_Crouch.IA_Crouch"))
  (bind _playerref (Variables|Default|GetPlayerRef))
  (:Started
    (Character|Crouch _playerref))
  (:Completed
    (Character|UnCrouch _playerref)))

(event Input|EnhancedActionEvents|EnhancedInputActionIA_Attack
  (params (ActionValue :type Boolean) (ElapsedSeconds :type Float%20%28double-precision%29) (TriggeredSeconds :type Float%20%28double-precision%29) (InputAction :type Input%20Action%20Object%20Reference :default "/Game/Assets/Input/Action/IA_Attack.IA_Attack"))
  (:Triggered
    (Default|CallAttackInput (Variables|Default|GetPlayerRef) :!label _label))
  (:Started
    (goto _label)))

(event EventBeginPlay
  (bind _self self)
  (bind _returnvalue (PlayerController|LocalPlayerSubsystems|GetEnhancedInputLocalPlayerSubsystem _self))
  (bind _asbp_player (Utilities|Casting|CastToBP_Player (Pawn|GetControlledPawn)))
  (Variables|Default|SetPlayerRef _asbp_player)
  (Utilities|IsValid _returnvalue
    (:Is%20Valid
      (Input|AddMappingContext _returnvalue "/Game/Assets/Input/IMC_Default.IMC_Default" 0 "(bIgnoreAllPressedKeysUntilRelease=True,bForceImmediately=False,bNotifyUserSettings=False)")
      (CallFunction|C2SCreateUI))))

(fn ConstructionScript)