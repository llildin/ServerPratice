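; BP_Player is the player character Blueprint that handles a networked attack action.
; Attack input is checked against the Idle or Move state locally, then again in the C2S event before it calls the S2M event.
; The S2M event sets the state to Attack and plays the attack montage on the mesh.
; A helper function returns the player state cast to BP_PlayerState.
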(event Custom|CallAttackInput
  (switch Utilities|FlowControl|Switch|SwitchonE_State (Variables|Default|GetState)
    (:NewEnumerator0
      (CallFunction|C2SAttack))))

(event Custom|C2S_Attack
  (switch Utilities|FlowControl|Switch|SwitchonE_State (Variables|Default|GetState)
    (:NewEnumerator0
      (CallFunction|S2MAttack))))

(event Custom|S2M_Attack
  (Utilities|FlowControl|Sequence
    (:then_0
      (Variables|Default|SetState "NewEnumerator1"))
    (:then_1
      (Animation|Montage|PlayMontage (Variables|Character|GetMesh) "/Game/Assets/Animations/AM_Attack.AM_Attack"))))

(fn ConstructionScript
  (|CallParentFunction))

(fn GetPlayerState
  (bind _asbp_player_state (Utilities|Casting|CastToBP_PlayerState (Variables|Default|GetPlayerState))
    (:then
      (return _asbp_player_state))
    (:CastFailed
      (return 0))))