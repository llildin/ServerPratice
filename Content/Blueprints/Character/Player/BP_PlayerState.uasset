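; BP_PlayerState is a player state Blueprint that keeps the HUD's HP display in step with its own lifetime.
; On BeginPlay it refreshes the display and binds to its OnDestroyed delegate, so the display refreshes again when it is destroyed.
; RefreshPlayerHp takes the HUD from player controller 0, casts it to BP_HUD and passes itself to RefreshHP.
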(event Custom|OnDestroyed_Event
  (params (DestroyedActor :type Actor%20Object%20Reference))
  (CallFunction|RefreshPlayerHp))

(event EventBeginPlay
  (CallFunction|RefreshPlayerHp)
  (Game|AssignOnDestroyed (delegate Custom|OnDestroyed_Event)))

(fn ConstructionScript)

(fn RefreshPlayerHp
  (bind _returnvalue (Game|GetPlayerController 0))
  (Utilities|IsValid _returnvalue
    (:Is%20Valid
      (bind _asbp_hud (Utilities|Casting|CastToBP_HUD (HUD|GetHUD _returnvalue)))
      (Default|RefreshHP _asbp_hud self))))